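; Woodcutter enemy that destroys Divinity Trees and triggers game over when its DivinityTreeLeft count reaches zero.
; AttackDivinityTree reads the target from the first AIC_WoodCutter found in the world, destroys it, updates the HUD count and calls CallAttackEnd.
; Game over shows the canvas, switches to UI-only input with a cursor and nearly freezes time through global dilation.
; Helper functions supply the patrol route, report it as non-interactable and map speed states to walk speed.
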(event `AttackDivinityTree`
  (bind _returnvalue (`GameplayStatics.GetPlayerController` 0))
  ; PlayerKilled
  (bind _returnvalue_2 (`GameplayStatics.GetActorOfClass` "/Game/Blueprint/IA/AIC_WoodCutter.AIC_WoodCutter_C"))
  (bind _asbp_divinity_tree (cast `/Game/Blueprint/BP_DivinityTree` (`BlackboardComponent.GetValueAsObject` (`AIBlueprintHelperLibrary.GetBlackboard` _returnvalue_2) "AttackTarget")))
  (`self.K2_DestroyActor` _asbp_divinity_tree)
  (bind _output_get (set `self.DivinityTreeLeft` (- (`self.DivinityTreeLeft`) 1)))
  (bind _asmain_hud (cast `/Game/UI/MainHUD` (`PlayerController.GetHUD` (`GameplayStatics.GetPlayerController` 0))))
  (bind _ui_reference (`/Game/UI/MainHUD.UI_Reference` _asmain_hud))
  (set `TextBlock.Text` (`KismetTextLibrary.Conv_IntToText` _output_get) (`/Game/UI/WBP_HUD.UI_DivinityTreeLeft` _ui_reference))
  (`self.AttackEnd`)
  (if (== (`self.DivinityTreeLeft`) 0)
    (set `Widget.Visibility` "Visible" (`/Game/UI/WBP_HUD.UI_CanvasGameOver` _ui_reference))
    (`WidgetBlueprintLibrary.SetInputMode_UIOnlyEx` _returnvalue null)
    (`GameplayStatics.SetGlobalTimeDilation` 0.01)
    (set `PlayerController.bShowMouseCursor` true _returnvalue)))

(fn `GetPatrolRoute`
  (returns (PatrolRoute :type "/Game/Blueprint/IA/BP_PatrolRoute Object Reference"))
  (return (`self.Patrol Route`)))

(fn `IsInteractable`
  (returns (Interactable :type Boolean))
  (return false))

(fn `SetMoveSpeed`
  (params (Speed :type "/Game/Blueprint/IA/Enums/E_MovementSpeed Enum" :default "NewEnumerator0"))
  (returns (SpeedValue :type "Float (double-precision)"))
  (bind _output_get (set `CharacterMovementComponent.MaxWalkSpeed` (select `/Game/Blueprint/IA/Enums/E_MovementSpeed` Speed :`NewEnumerator1` 100.0 :`NewEnumerator2` 200.0 :`NewEnumerator3` 340.0 :!type "Float (single-precision)") (`self.CharacterMovement`)))
  (return _output_get))

(fn `UserConstructionScript`)