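; Base game instance that holds game state: player position, spiritual-form flag, ethereal charges, and placed props and enemies.
; Save functions gather tagged actors into parallel class and location arrays, and load functions respawn from passed-in classes and stored locations.
; ClearEnemyPosition clears the placeable positions instead of the enemy ones.
; SetEtherealCharges is an empty stub, and LoadEnemiesPosition returns inside its spawn loop.
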(fn `ClearEnemyPosition`
  (`KismetArrayLibrary.Array_Clear` (`self.ArrayPlaceablePosition`)))

(fn `ClearEnemyTypes`
  (`KismetArrayLibrary.Array_Clear` (`self.ArrayEnemiesType`)))

(fn `ClearPlaceablePosition`
  (`KismetArrayLibrary.Array_Clear` (`self.ArrayPlaceablePosition`)))

(fn `ClearPlaceableTypes`
  (`KismetArrayLibrary.Array_Clear` (`self.ArrayPlaceableType`)))

(fn `LoadEnemiesPosition`
  (params (ArrayEnemiesClass :type "Array of Actor Class Reference"))
  (returns (ArrayTypesOutput :type "Array of Actor Class Reference") (ArrayPositionOutput :type "Array of Vector Structure"))
  (for (_array_element _array_index) ArrayEnemiesClass
    (bind _output (`|GetArrayItem` (`self.ArrayEnemiesPosition`) _array_index))
    (`|SpawnActorFromClass` _array_element (`KismetMathLibrary.Conv_VectorToTransform` _output) "Undefined" "MultiplyWithRoot" null null)
    (return (`|MakeArray` _array_element) (`|MakeArray` _output))))

(fn `LoadPlaceablePosition`
  (params (ArrayPlaceableClass :type "Array of Actor Class Reference"))
  (for (_array_element _array_index) ArrayPlaceableClass
    (`|SpawnActorFromClass` _array_element (`KismetMathLibrary.Conv_VectorToTransform` (`|GetArrayItem` (`self.ArrayPlaceablePosition`) _array_index)) "Undefined" "MultiplyWithRoot" null null)))

(fn `SaveActualForm`
  (params (Form :type Boolean))
  (set `self.IsInSpiritualForm` Form))

(fn `SaveEnemiesPosition`
  (params (EnemiesTag :type Name))
  (returns (ArrayEnemiesLocation :type "Array of Vector Structure"))
  (bind _outactors (`GameplayStatics.GetAllActorsWithTag` EnemiesTag))
  (for _array_element _outactors
    (`KismetArrayLibrary.Array_Add` (`self.ArrayEnemiesPosition`) (`Actor.K2_GetActorLocation` _array_element)))
  (return (`self.ArrayEnemiesPosition`)))

(fn `SaveEnemiesType`
  (params (EnemiesTag :type Name))
  (returns (ArrayType :type "Array of Actor Class Reference") (ArrayActors :type "Array of Actor Object Reference"))
  (bind _arrayenemiestype (`self.ArrayEnemiesType`))
  (bind _outactors (`GameplayStatics.GetAllActorsWithTag` EnemiesTag))
  (for _array_element _outactors
    (`KismetArrayLibrary.Array_Add` _arrayenemiestype (`GameplayStatics.GetObjectClass` _array_element)))
  (return _arrayenemiestype _outactors))

(fn `SaveEtherealCharges`
  (params (EtheralCharges :type Integer))
  (bind _output_get (set `self.ActualEtherealCharges` EtheralCharges))
  (`KismetSystemLibrary.PrintString` (`KismetStringLibrary.Concat_StrStr` "Saved! Actual Charges: " (`KismetStringLibrary.Conv_IntToString` _output_get))))

(fn `SavePlaceableNumber`
  (returns (`Number Of Item` :type Integer))
  (bind _outactors (`GameplayStatics.GetAllActorsWithTag` "ModularProp"))
  (for _ _outactors
    (set `self.Number Of Item` (+ (`self.Number Of Item`) 1)))
  (return (`self.Number Of Item`)))

(fn `SavePlaceablePosition`
  (params (ActorTag :type Name))
  (returns (ArrayPlaceableLocation :type "Array of Vector Structure"))
  (bind _outactors (`GameplayStatics.GetAllActorsWithTag` ActorTag))
  (for _array_element _outactors
    (`KismetArrayLibrary.Array_Add` (`self.ArrayPlaceablePosition`) (`Actor.K2_GetActorLocation` _array_element)))
  (return (`self.ArrayPlaceablePosition`)))

(fn `SavePlaceableType`
  (params (ActorTag :type Name))
  (returns (ArrayType :type "Array of Actor Class Reference"))
  (bind _outactors (`GameplayStatics.GetAllActorsWithTag` ActorTag))
  (for _array_element _outactors
    (`KismetArrayLibrary.Array_Add` (`self.ArrayPlaceableType`) (`GameplayStatics.GetObjectClass` _array_element)))
  (return (`self.ArrayPlaceableType`)))

(fn `SavePlayerPosition`
  (bind _returnvalue (`GameplayStatics.GetActorOfClass` "/Game/Blueprint/BP_Player.BP_Player_C"))
  (set `self.PlayerPosition` (`Actor.K2_GetActorLocation` _returnvalue)))

(fn `SetEtherealCharges`
  (params (EtherealCharges :type Integer))
  (return))