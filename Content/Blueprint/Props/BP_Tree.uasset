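; BP_Tree is a tree prop that tells the player when it is within reach of trees.
; Actor overlap begin and end set the CanReachTrees flag on BP_Player to true and false.
; The click event only looks up BP_ThirdPersonPlayerController and does nothing with it.
; A GetLocationClicked helper, not called here, returns hit status and location from a complex Visibility trace under the cursor.
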(event `self.ReceiveActorBeginOverlap`
  (params (OtherActor :type "Actor Object Reference"))
  (bind _asbp_player (cast `/Game/Blueprint/BP_Player` OtherActor))
  (set `/Game/Blueprint/BP_Player.CanReachTrees` true _asbp_player))

(event `self.ReceiveActorEndOverlap`
  (params (OtherActor :type "Actor Object Reference"))
  (bind _asbp_player (cast `/Game/Blueprint/BP_Player` OtherActor))
  (set `/Game/Blueprint/BP_Player.CanReachTrees` false _asbp_player))

(event `self.ReceiveActorOnClicked`
  (params (ButtonPressed :type "Key Structure"))
  (`GameplayStatics.GetActorOfClass` "/Game/Blueprint/BP_ThirdPersonPlayerController.BP_ThirdPersonPlayerController_C"))

(fn `GetLocationClicked`
  (returns (Hit :type Boolean) (Location :type "Vector Structure"))
  (bind (_bblockinghit _binitialoverlap _time _distance _location) (`GameplayStatics.BreakHitResult` (`PlayerController.GetHitResultUnderCursorByChannel` (`GameplayStatics.GetPlayerController` 0) "TraceTypeQuery1" true)))
  (return _bblockinghit _location))

(fn `UserConstructionScript`)