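; AI Controller for the Hunter enemy that reacts to seeing or hearing the player.
; On possession it runs BT_Hunter in the Passive state, then perception updates drive the Blackboard state, seen flag, target and point of interest.
; Sight switches Passive, Patrol or Investigate to Attacking; hearing without sight triggers Investigate only from Passive or Investigate.
; The perception handler also writes the Detected/Hidden indicator directly to the main HUD.
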(event `self.ReceivePossess`
  (params (PossessedPawn :type "Pawn Object Reference"))
  (`self.RunBehaviorTree` "/Game/Blueprint/IA/BT_Hunter.BT_Hunter")
  (`self.SetStateAsPassive`))

(event `self.AIPerception.OnPerceptionUpdated`
  (params (UpdatedActors :type "Array of Actor Object Reference (by ref)"))
  (for _array_element UpdatedActors
    (bind _sensed (`self.Can Sense Actor` _array_element "NewEnumerator1"))
    (if _sensed
      (bind _output_get (set `self.IsSeeingPlayer` true))
      (`self.SetIsSeeing` _output_get (`GameplayStatics.GetPlayerCharacter` 0))
      (bind _asmain_hud (cast `/Game/UI/MainHUD` (`PlayerController.GetHUD` (`GameplayStatics.GetPlayerController` 0))))
      (bind _uiref (`/Game/UI/WBP_HUD.UIRef` (`/Game/UI/MainHUD.UI_Reference` _asmain_hud)))
      (set `TextBlock.Text` "Detected" _uiref)
      (set `TextBlock.ColorAndOpacity` (make `SlateColor` (struct :`R` 1.0 :`G` 0.00827 :`A` 1.0)) _uiref)
      (`self.Handle Sense Sight Player` _array_element)
      (else
        (bind _output_get_2 (set `self.IsSeeingPlayer` false))
        (`self.SetIsSeeing` _output_get_2 (`GameplayStatics.GetPlayerCharacter` 0))
        (set `TextBlock.Text` "Hidden" _uiref)
        (set `TextBlock.ColorAndOpacity` (make `SlateColor` (struct :`G` 0.366253 :`B` 1.0 :`A` 0.701961)) _uiref)
        (bind (_sensed_2 _stimulus) (`self.Can Sense Actor` _array_element "NewEnumerator2"))
        (if _sensed_2
          (`self.Handle Sense Sound` (`.StimulusLocation` (break `AIStimulus` _stimulus))))))))

(fn `Can Sense Actor`
  (params (Actor :type "Actor Object Reference") (Sense :type "/Game/Blueprint/IA/Enums/E_AISense Enum" :default "NewEnumerator0"))
  (returns (Sensed :type Boolean) (Stimulus :type "AIStimulus Structure"))
  (if (`self.ActorHasTag` Actor "Player")
    (bind _info (`AIPerceptionComponent.GetActorsPerception` (`self.AIPerception`) Actor))
    (for _array_element (`.LastSensedStimuli` (break `ActorPerceptionBlueprintInfo` _info))
      (bind _returnvalue (`AIPerceptionSystem.GetSenseClassForStimulus` _array_element))
      (if (== _returnvalue (select `/Game/Blueprint/IA/Enums/E_AISense` Sense :`NewEnumerator1` "/Script/AIModule.AISense_Sight" :`NewEnumerator2` "/Script/AIModule.AISense_Hearing" :!type "Object Class Reference"))
        (return (`.bSuccessfullySensed` (break `AIStimulus` _array_element)) _array_element)))))

(fn `Get Current State`
  (returns (NewParam :type "/Game/Blueprint/IA/Enums/E_EnemyState Enum"))
  (return (cast `/Game/Blueprint/IA/Enums/E_EnemyState` (`BlackboardComponent.GetValueAsEnum` (`self.Blackboard`) (`self.State Key Name`)))))

(fn `Handle Sense Sight Player`
  (params (Actor :type "Actor Object Reference"))
  (bind _returnvalue (`GameplayStatics.GetPlayerCharacter` 0))
  (bind _newparam (`self.Get Current State`))
  (switch `/Game/Blueprint/IA/Enums/E_EnemyState` _newparam
    (:`NewEnumerator0`
      _)
    (:`NewEnumerator1`
      _)
    (:`NewEnumerator3`
      _))
  (if (== Actor _returnvalue)
    (`self.SetStateAsAttacking` _returnvalue)))

(fn `Handle Sense Sound`
  (params (Location :type "Vector Structure"))
  (bind _newparam (`self.Get Current State`))
  (switch `/Game/Blueprint/IA/Enums/E_EnemyState` _newparam
    (:`NewEnumerator0`
      _)
    (:`NewEnumerator3`
      _))
  (`self.Set State As Investigating` Location))

(fn `Set State As Investigating`
  (params (Location :type "Vector Structure"))
  (bind _blackboard (`self.Blackboard`))
  (`BlackboardComponent.SetValueAsEnum` _blackboard (`self.EnemyStateKey`) (enumliteral `/Game/Blueprint/IA/Enums/E_EnemyState` "NewEnumerator3"))
  (`BlackboardComponent.SetValueAsVector` _blackboard (`self.Point Of Interest Key Name`) Location))

(fn `SetIsSeeing`
  (params (`See?` :type Boolean) (Target :type "Actor Object Reference"))
  (`BlackboardComponent.SetValueAsBool` (`self.Blackboard`) (`self.Key Name`) `See?`))

(fn `SetStateAsAttacking`
  (params (`Attack Target` :type "Actor Object Reference"))
  (`BlackboardComponent.SetValueAsObject` (`self.Blackboard`) (`self.AttackTargetKeyName`) `Attack Target`)
  (`BlackboardComponent.SetValueAsEnum` (`self.Blackboard`) (`self.EnemyStateKey`) (enumliteral `/Game/Blueprint/IA/Enums/E_EnemyState` "NewEnumerator2")))

(fn `SetStateAsPassive`
  (`BlackboardComponent.SetValueAsEnum` (`self.Blackboard`) (`self.EnemyStateKey`) (enumliteral `/Game/Blueprint/IA/Enums/E_EnemyState` "NewEnumerator0")))

(fn `UserConstructionScript`)