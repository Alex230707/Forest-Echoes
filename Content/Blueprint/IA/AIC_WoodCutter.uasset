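; AI controller for the woodcutter enemy, which runs BT_WoodCutter and starts it in the Passive state.
; Perception updates check sight first, switching a non-attacking woodcutter to Attacking when it sees an actor tagged DivinityTree.
; Otherwise, heard sounds move Passive or Investigate states to investigating that location.
; State, target and point of interest go through the Blackboard; AffectMimetization reads the player's MimetizationLevel but acts on nothing.
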(event `AffectMimetization`
  (bind _returnvalue (`GameplayStatics.GetActorOfClass` "/Game/Blueprint/BP_Player.BP_Player_C"))
  (switch `int` (`/Game/Blueprint/BP_Player.MimetizationLevel` _returnvalue)))

(event `self.ReceivePossess`
  (params (PossessedPawn :type "Pawn Object Reference"))
  (`self.RunBehaviorTree` "/Game/Blueprint/IA/BT_WoodCutter.BT_WoodCutter")
  (`self.SetStateAsPassive`))

(event `self.AIPerception.OnPerceptionUpdated`
  (params (UpdatedActors :type "Array of Actor Object Reference (by ref)"))
  (for _array_element UpdatedActors
    (bind _sensed (`self.Can Sense Actor` _array_element "NewEnumerator1"))
    (if _sensed
      (set `self.IsSeeingDivinityTree` true)
      (`self.Handle Sense Sight Divinity Tree` _array_element)
      (else
        (set `self.IsSeeingDivinityTree` false)
        (bind (_sensed_2 _stimulus) (`self.Can Sense Actor` _array_element "NewEnumerator2"))
        (if _sensed_2
          (`self.Handle Sense Sound` (`.StimulusLocation` (break `AIStimulus` _stimulus))))))))

(fn `Can Sense Actor`
  (params (Actor :type "Actor Object Reference") (Sense :type "/Game/Blueprint/IA/Enums/E_AISense Enum" :default "NewEnumerator0"))
  (returns (Sensed :type Boolean) (Stimulus :type "AIStimulus Structure"))
  (bind _info (`AIPerceptionComponent.GetActorsPerception` (`self.AIPerception`) Actor))
  (for _array_element (`.LastSensedStimuli` (break `ActorPerceptionBlueprintInfo` _info))
    (bind _returnvalue (`AIPerceptionSystem.GetSenseClassForStimulus` _array_element))
    (if (== _returnvalue (select `/Game/Blueprint/IA/Enums/E_AISense` Sense :`NewEnumerator1` "/Script/AIModule.AISense_Sight" :`NewEnumerator2` "/Script/AIModule.AISense_Hearing" :!type "Object Class Reference"))
      (return (`.bSuccessfullySensed` (break `AIStimulus` _array_element)) _array_element))))

(fn `Get Current State`
  (returns (NewParam :type "/Game/Blueprint/IA/Enums/E_EnemyState Enum"))
  (return (cast `/Game/Blueprint/IA/Enums/E_EnemyState` (`BlackboardComponent.GetValueAsEnum` (`self.Blackboard`) (`self.State Key Name`)))))

(fn `Handle Sense Sight Divinity Tree`
  (params (Actor :type "Actor Object Reference"))
  (bind _newparam (`self.Get Current State`))
  (switch `/Game/Blueprint/IA/Enums/E_EnemyState` _newparam
    (:`NewEnumerator0`
      _)
    (:`NewEnumerator1`
      _)
    (:`NewEnumerator3`
      _))
  (if (`self.ActorHasTag` Actor "DivinityTree")
    (`self.SetStateAsAttacking` Actor)))

(fn `Handle Sense Sound`
  (params (Location :type "Vector Structure"))
  (bind _newparam (`self.Get Current State`))
  (switch `/Game/Blueprint/IA/Enums/E_EnemyState` _newparam
    (:`NewEnumerator0`
      _)
    (:`NewEnumerator3`
      _))
  (`self.Set State As Investigating` Location))

(fn `Set State As Investigating`
  (params (Location :type "Vector Structure"))
  (bind _blackboard (`self.Blackboard`))
  (`BlackboardComponent.SetValueAsEnum` _blackboard (`self.EnemyStateKey`) (enumliteral `/Game/Blueprint/IA/Enums/E_EnemyState` "NewEnumerator3"))
  (`BlackboardComponent.SetValueAsVector` _blackboard (`self.Point Of Interest Key Name`) Location))

(fn `SetStateAsAttacking`
  (params (`Attack Target` :type "Actor Object Reference"))
  (`BlackboardComponent.SetValueAsObject` (`self.Blackboard`) (`self.AttackTargetKeyName`) `Attack Target`)
  (`BlackboardComponent.SetValueAsEnum` (`self.Blackboard`) (`self.EnemyStateKey`) (enumliteral `/Game/Blueprint/IA/Enums/E_EnemyState` "NewEnumerator2")))

(fn `SetStateAsPassive`
  (`BlackboardComponent.SetValueAsEnum` (`self.Blackboard`) (`self.EnemyStateKey`) (enumliteral `/Game/Blueprint/IA/Enums/E_EnemyState` "NewEnumerator0")))

(fn `UserConstructionScript`)