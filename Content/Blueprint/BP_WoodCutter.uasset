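; BP_WoodCutter is an enemy AI character that attacks the player and can trigger game over.
; Attack removes one health from BP_Player, updates the HUD life text, then signals attack end after a delay.
; At zero health it shows the game-over UI with retry and quit, switches to UI-only input and slows time.
; Helper functions expose a patrol route, report it non-interactable, and map movement states to walk speeds.
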(event `Attack`
  (bind _returnvalue (`GameplayStatics.GetPlayerController` 0))
  ; PlayerKilled
  (bind _returnvalue_2 (`GameplayStatics.GetActorOfClass` "/Game/Blueprint/BP_Player.BP_Player_C"))
  (bind _returnvalue_3 (- (`/Game/Blueprint/BP_Player.Health` _returnvalue_2) 1))
  (bind _output_get (set `/Game/Blueprint/BP_Player.Health` _returnvalue_3 _returnvalue_2))
  (bind _asmain_hud (cast `/Game/Blueprint/UI/MainHUD` (`PlayerController.GetHUD` (`GameplayStatics.GetPlayerController` 0))))
  (if (== _returnvalue_3 -1)
    (bind _ui_reference (`/Game/Blueprint/UI/MainHUD.UI_Reference` _asmain_hud))
    (set `Widget.Visibility` "Visible" (`/Game/Blueprint/UI/WBP_HUD.UI_GameOver` _ui_reference))
    (set `Widget.Visibility` "Visible" (`/Game/Blueprint/UI/WBP_HUD.UI_ButtonRiprova` _ui_reference))
    (set `Widget.Visibility` "Visible" (`/Game/Blueprint/UI/WBP_HUD.UI_ButtonQuit` _ui_reference))
    (set `Widget.Visibility` "Hidden" (`/Game/Blueprint/UI/WBP_HUD.PressFToKill` _ui_reference))
    (set `Widget.Visibility` "Visible" (`/Game/Blueprint/UI/WBP_HUD.UI_CanvasGameOver` _ui_reference))
    (`WidgetBlueprintLibrary.SetInputMode_UIOnlyEx` _returnvalue null)
    (`GameplayStatics.SetGlobalTimeDilation` 0.03)
    (set `self.GameOver` true)
    (set `PlayerController.bShowMouseCursor` true _returnvalue))
  (set `TextBlock.Text` (`KismetTextLibrary.Conv_StringToText` (`KismetStringLibrary.Conv_IntToString` _output_get)) (`/Game/Blueprint/UI/WBP_HUD.UI_LifePoints` _ui_reference))
  (`KismetSystemLibrary.Delay` 1.0)
  (`self.AttackEnd`))

(fn `GetPatrolRoute`
  (returns (PatrolRoute :type "/Game/Blueprint/IA/BP_PatrolRoute Object Reference"))
  (return (`self.Patrol Route`)))

(fn `IsInteractable`
  (returns (Interactable :type Boolean))
  (return false))

(fn `SetMoveSpeed`
  (params (Speed :type "/Game/Blueprint/IA/Enums/E_MovementSpeed Enum" :default "NewEnumerator0"))
  (returns (SpeedValue :type "Float (double-precision)"))
  (bind _output_get (set `CharacterMovementComponent.MaxWalkSpeed` (select `/Game/Blueprint/IA/Enums/E_MovementSpeed` Speed :`NewEnumerator1` 100.0 :`NewEnumerator2` 200.0 :`NewEnumerator3` 340.0 :!type "Float (single-precision)") (`self.CharacterMovement`)))
  (return _output_get))

(fn `UserConstructionScript`)