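; Trigger box that marks foliage where the player's mimetization (camouflage) level rises while standing on grass.
; Box overlap sets the player's IsOnGrass flag and adds one level on entry, and end overlap clears it and subtracts one, with the flag guarding against repeats.
; Entry alone also calls AffectMimetization on the AIC_Hunter found in the world.
; Both paths share one update of the MainHUD mimetization text.
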(event `self.Box.OnComponentBeginOverlap`
  (params (OverlappedComponent :type "PrimitiveComponent Object Reference") (OtherActor :type "Actor Object Reference") (OtherComp :type "PrimitiveComponent Object Reference") (OtherBodyIndex :type Integer) (bFromSweep :type Boolean) (SweepResult :type "HitResult Structure (by ref)"))
  (bind _asbp_player (cast `/Game/Blueprint/BP_Player` OtherActor))
  (if (not (`/Game/Blueprint/BP_Player.IsOnGrass` _asbp_player))
    (bind _returnvalue (`GameplayStatics.GetActorOfClass` "/Game/Blueprint/IA/AIC_Hunter.AIC_Hunter_C"))
    (`/Game/Blueprint/IA/AIC_Hunter.AffectMimetization` _returnvalue)
    (set `/Game/Blueprint/BP_Player.IsOnGrass` true _asbp_player)
    (set `/Game/Blueprint/BP_Player.MimetizationLevel` (+ (`/Game/Blueprint/BP_Player.MimetizationLevel` _asbp_player) 1) _asbp_player)
    (bind _asmain_hud (cast `/Game/UI/MainHUD` (`PlayerController.GetHUD` (`GameplayStatics.GetPlayerController` 0)) :!label _label))
    (set `TextBlock.Text` (`KismetTextLibrary.Conv_IntToText` (`/Game/Blueprint/BP_Player.MimetizationLevel` _asbp_player)) (`/Game/UI/WBP_HUD.UI_TextMimetization` (`/Game/UI/MainHUD.UI_Reference` _asmain_hud)))))

(event `self.Box.OnComponentEndOverlap`
  (params (OverlappedComponent :type "PrimitiveComponent Object Reference") (OtherActor :type "Actor Object Reference") (OtherComp :type "PrimitiveComponent Object Reference") (OtherBodyIndex :type Integer))
  (bind _asbp_player (cast `/Game/Blueprint/BP_Player` OtherActor))
  (if (`/Game/Blueprint/BP_Player.IsOnGrass` _asbp_player)
    (set `/Game/Blueprint/BP_Player.IsOnGrass` false _asbp_player)
    (set `/Game/Blueprint/BP_Player.MimetizationLevel` (- (`/Game/Blueprint/BP_Player.MimetizationLevel` _asbp_player) 1) _asbp_player)
    (goto _label)))

(fn `UserConstructionScript`)